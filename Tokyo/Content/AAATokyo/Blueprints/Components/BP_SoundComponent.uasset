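; Actor component that plays positional footstep sounds for the left and right feet of its owner.
; On BeginPlay, Init finds each foot's scene component on the owner by a configurable tag and caches it.
; StepLeft and StepRight play the configured sound at that foot's world location with shared volume, pitch and step attenuation, skipping if the foot or sound is invalid.
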(event EventBeginPlay
  (Private|Init))

(fn StepLeft
  (Utilities|IsValid (Variables|Default|GetLeftFoot)
    (:Is%20Valid
      (Utilities|IsValid (Variables|Default|GetSound)
        (:Is%20Valid
          (Audio|PlaySoundatLocation (Variables|Default|GetSound) (Transformation|GetWorldLocation (Variables|Default|GetLeftFoot)) "0, 0, 0" (Variables|Default|GetVolume) (Variables|Default|GetPitch) 0.0 "/Game/AAATokyo/Sounds/FootstepsMiniPack/SA_Step.SA_Step" 0 (Components|GetOwner) 0))))))

(fn StepRight
  (Utilities|IsValid (Variables|Default|GetRightFoot)
    (:Is%20Valid
      (Utilities|IsValid (Variables|Default|GetSound)
        (:Is%20Valid
          (Audio|PlaySoundatLocation (Variables|Default|GetSound) (Transformation|GetWorldLocation (Variables|Default|GetRightFoot)) "0, 0, 0" (Variables|Default|GetVolume) (Variables|Default|GetPitch) 0.0 "/Game/AAATokyo/Sounds/FootstepsMiniPack/SA_Step.SA_Step" 0 (Components|GetOwner) 0))))))

(fn Init
  (Variables|Default|SetLeftFoot (Class|Actor|FindComponentbyTag (Components|GetOwner) "/Script/Engine.SceneComponent" (Variables|Default|GetTagLeftFoot)))
  (Variables|Default|SetRightFoot (Class|Actor|FindComponentbyTag (Components|GetOwner) "/Script/Engine.SceneComponent" (Variables|Default|GetTagRightFoot))))