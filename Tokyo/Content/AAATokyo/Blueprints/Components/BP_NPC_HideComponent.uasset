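; An NPC component that hides its owning Character's mesh while another Character overlaps it.
; On BeginPlay it caches the mesh and binds to the capsule's begin and end overlap events.
; Begin overlap hides the mesh and end overlap shows it, without propagating to child components.
; Overlaps are not counted, so any Character leaving restores visibility even if others still overlap.
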(event Custom|OnComponentBeginOverlap_Event
  (params (OverlappedComponent :type Primitive%20Component%20Object%20Reference) (OtherActor :type Actor%20Object%20Reference) (OtherComp :type Primitive%20Component%20Object%20Reference) (OtherBodyIndex :type Integer) (bFromSweep :type Boolean) (SweepResult :type Hit%20Result%20Structure%20%28by%20ref%29))
  (Utilities|Casting|CastToCharacter OtherActor)
  (Rendering|SetVisibility (Variables|Default|GetSkeletalMeshComponent) false false))

(event Custom|OnComponentEndOverlap_Event
  (params (OverlappedComponent :type Primitive%20Component%20Object%20Reference) (OtherActor :type Actor%20Object%20Reference) (OtherComp :type Primitive%20Component%20Object%20Reference) (OtherBodyIndex :type Integer))
  (Utilities|Casting|CastToCharacter OtherActor)
  (Rendering|SetVisibility (Variables|Default|GetSkeletalMeshComponent) true false))

(event EventBeginPlay
  (bind _ascharacter (Utilities|Casting|CastToCharacter (Components|GetOwner)))
  (Variables|Default|SetSkeletalMeshComponent (Variables|/Script/Engine.Character|GetMesh _ascharacter))
  (Collision|AssignOnComponentBeginOverlap (Variables|/Script/Engine.Character|GetCapsuleComponent _ascharacter) (delegate Custom|OnComponentBeginOverlap_Event))
  (Collision|AssignOnComponentEndOverlap (Variables|/Script/Engine.Character|GetCapsuleComponent _ascharacter) (delegate Custom|OnComponentEndOverlap_Event)))

(event EventTick
  (params (DeltaSeconds :type Float%20%28single-precision%29)))